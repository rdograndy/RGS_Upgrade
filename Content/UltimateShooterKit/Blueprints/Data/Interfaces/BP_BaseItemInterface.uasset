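; Blueprint Interface for items in the Ultimate Shooter Kit, declaring the shared calls other systems make on any item without knowing its class.
; It covers item info, meshes and data table, ownership, visibility and highlighting, attachment updates and resets, and on-item widget creation and removal.
; It also exposes weapon-oriented calls for fire mode, current clip and adding projectile movement.
; All functions are empty signatures, so implementing classes supply the behaviour.
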(fn GetItemMeshComponents
  (return 0 0))

(fn GetItemInfo
  (return "" ""))

(fn GetItemClassReference
  (return 0))

(fn UpdateDataTable
  (params (NewDataTable :type Data%20Table%20Row%20Handle%20Structure))
  (return false))

(fn UpdateVisibilityOfItem
  (params (OnlyOwnerSee :type Boolean) (OwnerNoSee :type Boolean) (CastShadow :type Boolean))
  (return false))

(fn UpdateHasOwner
  (params (HasOwner :type Boolean))
  (return false))

(fn GetCurrentAttachments
  (return 0))

(fn CreateWidgetonItem
  (params (WidgetInformation :type Struct%20Available%20Attachments%20Structure))
  (return 0))

(fn DestroyAllWidgetsonItem
  (return false))

(fn OnWidgetDestroyed
  (params (WidgetReference :type Widget%20Object%20Reference))
  (return false))

(fn UpdateCurrentAttachment
  (params (AttachmentInfo :type Struct%20Master%20Attachment%20Structure))
  (return false))

(fn ResetAttachmenttoDefault
  (params (AttachmentType :type Enum_AttachmentTypes%20Enum :default "NewEnumerator0"))
  (return false))

(fn UpdateHighlight
  (params (Highlighted :type Boolean))
  (return false))

(fn DestroyHoverWidget
  (return false))

(fn UpdateMasterItemInfo
  (params (NewItemInfo :type Struct%20Master%20Item%20Structure))
  (return))

(fn AddProjectileMovement)

(fn UpdateFireMode)

(fn GetFireMode
  (return "NewEnumerator0"))

(fn UpdateCurrentClip
  (params (Increase :type Boolean) (Amount :type Integer)))

(fn GetCurrentClip
  (return 0))