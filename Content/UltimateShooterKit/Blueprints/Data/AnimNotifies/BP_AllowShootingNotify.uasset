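; An animation notify, shown as "Shooting Handler", that sets whether the owning character's shooter component allows shooting at a point in an animation.
; On a locally controlled BP_TFPCharacter, it passes its ShootingIsAllowed value to Component_Shooter and clears the character's IsReloading flag.
; It then resets AnimInt on the ShooterOverlay anim instance to zero.
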(fn ReceivedNotify
  (params (MeshComp :type Skeletal%20Mesh%20Component%20Object%20Reference) (Animation :type Anim%20Sequence%20Base%20Object%20Reference))
  (bind _returnvalue (Components|GetOwner MeshComp))
  (bind _aspawn (Utilities|Casting|CastToPawn _returnvalue))
  (bind _asbp_tfpcharacter (Utilities|Casting|CastToBP_TFPCharacter _returnvalue))
  (Utilities|IsValid (Pawn|GetController _aspawn)
    (:Is%20Valid
      (if (Pawn|IsLocalController (Pawn|GetController _aspawn))
        (Default|SetAllowShooting (Actor|GetComponentbyClass _aspawn "/Game/UltimateShooterKit/Blueprints/Components/Component_Shooter.Component_Shooter_C") (Variables|Default|GetShootingIsAllowed?))
        (Variables|/Game/UltimateShooterKit/Blueprints/BP_TFPCharacter.BP_TFPCharacter_C|SetIsReloading _asbp_tfpcharacter false)
        (bind _asshooter_overlay_anim_bp (Utilities|Casting|CastToShooterOverlay_AnimBP (Default|GetOverlayAnimInstance (Actor|GetComponentbyClass _aspawn "/Game/UltimateShooterKit/Blueprints/Components/Component_Shooter.Component_Shooter_C") "ShooterOverlay")))
        (Variables|/Game/UltimateShooterKit/Blueprints/ShooterOverlay_AnimBP.ShooterOverlay_AnimBP_C|SetAnimInt _asshooter_overlay_anim_bp 0)
        (return true)))))

(fn GetNotifyName
  (return "Shooting Handler"))